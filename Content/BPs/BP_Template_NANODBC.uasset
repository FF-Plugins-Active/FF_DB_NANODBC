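; Template Blueprint that tests the NANODBC plugin by connecting to an ODBC database and printing query results on screen.
; On BeginPlay it spawns a NANODBC_Manager and opens a connection using server and credentials from the GI_Plugins game instance.
; If that succeeds, it selects last_login from a test table and prints each row's column type, name and preview.
; The insert function is unwired and executes an empty query.
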(event `self.ReceiveBeginPlay`
  (bind _returnvalue (`|SpawnActorFromClass` "/Script/FF_DB_NANODBC.NANODBC_Manager" (`KismetMathLibrary.MakeTransform` (0.0 0.0 0.0)) "Undefined" "MultiplyWithRoot" null null))
  (set `self.NANODBC_Manager` _returnvalue)
  (bind _asgi_plugins (cast `/Game/Player/GI_Plugins` (`GameplayStatics.GetGameInstance`)))
  (bind (_out_code _createdconnection _returnvalue_2) (`NANODBC_Manager.NANODBC_Connection_Create` (`self.NANODBC_Manager`) (`BlueprintMapLibrary.Map_Find` (`/Game/Player/GI_Plugins.ODBC_Servers` _asgi_plugins) "home") (`BlueprintMapLibrary.Map_Find` (`/Game/Player/GI_Plugins.Users` _asgi_plugins) "odbc") (`BlueprintMapLibrary.Map_Find` (`/Game/Player/GI_Plugins.Passwords` _asgi_plugins) "odbc")))
  (`KismetSystemLibrary.PrintString` _out_code true true (`KismetMathLibrary.SelectColor` (struct :`G` 1.0 :`A` 1.0) (struct :`R` 1.0 :`A` 1.0) _returnvalue_2) 30.0)
  (if _returnvalue_2
    (set `self.NANODBC_Connection` _createdconnection)
    (`self.F_Data_View`)))

(fn `F_Data_Insert`
  (locals (LOC_Result :type "NANODBC_Result Object Reference"))
  (bind (_out_code _returnvalue) (`NANODBC_Connection.JustExecute` (`self.NANODBC_Connection`) ""))
  (`KismetSystemLibrary.PrintString` _out_code true true (`KismetMathLibrary.SelectColor` (struct :`G` 1.0 :`A` 1.0) (struct :`R` 1.0 :`A` 1.0) _returnvalue) 30.0)
  (return))

(fn `F_Data_View`
  (locals (LOC_Result :type "NANODBC_Result Object Reference"))
  (bind (_out_code _out_result _returnvalue) (`NANODBC_Connection.ExecuteAndGetResult` (`self.NANODBC_Connection`) "SELECT last_login FROM ue5_test.dbo.Table_1"))
  (`KismetSystemLibrary.PrintString` _out_code true true (`KismetMathLibrary.SelectColor` (struct :`G` 1.0 :`A` 1.0) (struct :`R` 1.0 :`A` 1.0) _returnvalue) 30.0)
  (if _returnvalue
    (set `local.LOC_Result` _out_result)
    (for _index (range (`.ReturnValue` (`NANODBC_Result.GetRowsCount` (`local.LOC_Result`))))
      (bind (_out_code_2 _out_value _returnvalue_2) (`NANODBC_Result.GetDataFromRow` (`local.LOC_Result`) _index))
      (if _returnvalue_2
        (bind _out_row (`self.F_Recurse_Row` _out_value " // "))
        (`KismetSystemLibrary.PrintString` _out_row true true (struct :`G` 0.66 :`B` 1.0 :`A` 1.0) 60.0)
        (else
          (`KismetSystemLibrary.PrintString` _out_code_2 true true (struct :`G` 0.66 :`B` 1.0 :`A` 1.0) 30.0))))
    (return)
    (else
      (return))))

(fn `F_Recurse_Row`
  (params (In_Row :type "Array of NANODBC_DataValue Structure") (Separator :type String :default " = "))
  (returns (Out_Row :type String))
  (locals (Each_Row :type "Array of String"))
  (for _array_element In_Row
    (`KismetArrayLibrary.Array_Add` (`local.Each_Row`) (`KismetStringLibrary.Concat_StrStr` (`KismetStringLibrary.Conv_IntToString` (`.DataType` (break `NANODBC_DataValue` _array_element))) " = " (`.DataTypeName` (break `NANODBC_DataValue` _array_element)) " = " (`.ColumnName` (break `NANODBC_DataValue` _array_element)) " = " (`.Preview` (break `NANODBC_DataValue` _array_element)))))
  (return (`KismetStringLibrary.JoinStringArray` (`local.Each_Row`) Separator)))

(fn `UserConstructionScript`)